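; MyEnemy_BP is a melee enemy Blueprint exposing Walk, Run and Attack events; their callers are not in this file.
; Walk and Run set movement speed, and Run also starts a walk animation, then immediately restores Animation Blueprint mode.
; Attack plays a one-shot attack animation directly on the mesh, holds the Attacking flag for a fixed delay, then returns the mesh to its Animation Blueprint.
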(event Custom|Walk
  (Variables|/Script/Engine.CharacterMovementComponent|SetMaxWalkSpeed (Variables|Character|GetCharacterMovement) 1.5e+02))

(event Custom|Run
  (Variables|/Script/Engine.CharacterMovementComponent|SetMaxWalkSpeed (Variables|Character|GetCharacterMovement) 4e+02)
  (Components|Animation|PlayAnimation (Variables|Character|GetMesh) "/Game/Enemy_Melee_Walk_Anim.Enemy_Melee_Walk_Anim" false)
  (Components|Animation|SetAnimationMode (Variables|Character|GetMesh) "AnimationBlueprint"))

(event Custom|Attack
  (Components|Animation|PlayAnimation (Variables|Character|GetMesh) "/Game/Enemy_Melee_Atk1_Anim.Enemy_Melee_Atk1_Anim" false)
  (Variables|Default|SetAttacking true)
  (Utilities|FlowControl|Delay 1.5)
  (Variables|Default|SetAttacking false)
  (Components|Animation|SetAnimationMode (Variables|Character|GetMesh) "AnimationBlueprint"))

(fn ConstructionScript)