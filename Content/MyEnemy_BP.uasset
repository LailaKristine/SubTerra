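; Enemy character Blueprint that exposes Walk, Run and Attack events, with no logic in this file that triggers them.
; Walk and Run switch the movement component's max speed between a slow and a fast value.
; Attack plays a one-shot animation directly on the mesh and holds an Attacking flag for a fixed delay, then returns the mesh to Animation Blueprint mode.
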(event Custom|Walk
  (Variables|/Script/Engine.CharacterMovementComponent|SetMaxWalkSpeed (Variables|Character|GetCharacterMovement) 1.5e+02))

(event Custom|Run
  (Variables|/Script/Engine.CharacterMovementComponent|SetMaxWalkSpeed (Variables|Character|GetCharacterMovement) 4e+02))

(event Custom|Attack
  (Components|Animation|PlayAnimation (Variables|Character|GetMesh) 0 false)
  (Variables|Default|SetAttacking true)
  (Utilities|FlowControl|Delay 1.5)
  (Variables|Default|SetAttacking false)
  (Components|Animation|SetAnimationMode (Variables|Character|GetMesh) "AnimationBlueprint"))

(fn ConstructionScript)