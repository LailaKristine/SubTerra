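; AI controller for MyEnemy_BP that runs the Tree_BP behavior tree and gathers TargetPoints tagged "Tut" as patrol points on possession.
; AI perception updates the blackboard's player visibility, saving the player's location and a recently-sighted flag when sight is lost.
; GetNewPoint writes a random patrol point to the blackboard, while Walk, Run and Attack events forward to the possessed enemy.
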(event OnTargetPerceptionUpdated(AIPerception)
  (params (Actor :type Actor%20Object%20Reference) (Stimulus :type AI%20Stimulus%20Structure))
  (bind _bsuccessfullysensed (Utilities|Struct|BreakAIStimulus Stimulus))
  (bind _returnvalue (AI|GetBlackboard 0))
  (Utilities|Casting|CastToPlayer Actor)
  (AI|Components|Blackboard|SetValueasBool _returnvalue (Utilities|Name|MakeLiteralName "CanSeePlayer") _bsuccessfullysensed)
  (if (not _bsuccessfullysensed)
    (AI|Components|Blackboard|SetValueasVector _returnvalue (Utilities|Name|MakeLiteralName "PlayerLocation") (Transformation|GetActorLocation (Game|GetPlayerCharacter 0)))
    (AI|Components|Blackboard|SetValueasBool _returnvalue (Utilities|Name|MakeLiteralName "RecentlySighted") true)))

(event Custom|Walk
  (Default|Walk (Variables|Default|GetEnemy)))

(event Custom|Run
  (Default|Run (Variables|Default|GetEnemy)))

(event Custom|GetNewPoint
  (bind _patrolpoints (Variables|Default|GetPatrolPoints))
  (AI|Components|Blackboard|SetValueasObject (AI|GetBlackboard 0) (Utilities|Name|MakeLiteralName "TargetPointKey") (Utilities|Array|Get(acopy) _patrolpoints (Math|Random|RandomIntegerinRange 0 (- (Utilities|Array|Length _patrolpoints) 1)))))

(event Custom|Attack
  (Default|Attack (Variables|Default|GetEnemy)))

(event EventOnPossess
  (params (PossessedPawn :type Pawn%20Object%20Reference))
  (bind _asmy_enemy_bp (Utilities|Casting|CastToMyEnemy_BP PossessedPawn))
  (Variables|Default|SetEnemy _asmy_enemy_bp)
  (AI|RunBehaviorTree "/Game/Tree_BP.Tree_BP")
  (bind _outactors (Actor|GetAllActorsOfClass "/Script/Engine.TargetPoint"))
  (for _array_element _outactors
    (if (Actor|ActorHasTag _array_element "Tut")
      (Utilities|Array|Add (Variables|Default|GetPatrolPoints) _array_element))))

(fn ConstructionScript)